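; Grid entity actor that moves to a target grid cell and its world position.
; MovetoGridCoords stores the target coords as CurrentPosition, then plays a timeline that lerps from the actor's current location each update, without sweep.
; The timeline also switches CharacterState on the first BP_PlayerEntity found, whichever entity is moving, during and after the move.
; GetGridCoords and the other events hold no logic.
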(event `self.ReceiveBeginPlay`)

(event `/Game/Blueprints/Interfaces/BPI_GridPawn.MoveToGridCoords`
  (params (TargetCoords :type "IntPoint Structure") (TargetWorldLocation :type "Vector Structure"))
  (bind _returnvalue (`GameplayStatics.GetActorOfClass` "/Game/Blueprints/BP_PlayerEntity.BP_PlayerEntity_C"))
  (set `self.ControlledPawn` _returnvalue)
  (set `self.CurrentPosition` TargetCoords)
  (bind (_direction _newtrack_0) (`Timeline|MoveTimeline` :!via `PlayFromStart`)
    (:`Update`
      (set `/Game/Blueprints/BP_PlayerEntity.CharacterState` "NewEnumerator1" (`self.ControlledPawn`))
      (`self.K2_SetActorLocation` (`KismetMathLibrary.VLerp` (`self.K2_GetActorLocation`) TargetWorldLocation _newtrack_0)))
    (:`Finished`
      (set `/Game/Blueprints/BP_PlayerEntity.CharacterState` "NewEnumerator0" (`self.ControlledPawn`)))))

(fn `GetGridCoords`
  (returns (Coords :type "IntPoint Structure"))
  (return))

(fn `UserConstructionScript`)