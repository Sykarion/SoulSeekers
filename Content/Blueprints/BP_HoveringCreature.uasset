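; Hovering creature actor that moves on a sine wave over game time.
; BeginPlay stores its starting Z and shifts the world origin to the actor's truncated location, then runs the same movement step as Tick.
; That step offsets the stored Z by a sine scaled with HoverSpeed and HoverHeight.
; The resulting float converts directly to a vector, so X, Y and Z all receive that value.
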(event `self.ReceiveBeginPlay`
  (bind _returnvalue (`self.K2_GetActorLocation`))
  (bind _output_get (set `self.BaseZLocation` (.z _returnvalue)))
  (`GameplayStatics.SetWorldOriginLocation` (`KismetMathLibrary.FTruncVector` _returnvalue))
  (`self.K2_SetActorLocation` (`KismetMathLibrary.Conv_DoubleToVector` (+ _output_get (* (`KismetMathLibrary.Sin` (* (`KismetSystemLibrary.GetGameTimeInSeconds`) (`self.HoverSpeed`))) (`self.HoverHeight`)))) :!label _label))

(event `self.ReceiveTick`
  (params (DeltaSeconds :type "Float (single-precision)"))
  (goto _label))

(fn `UserConstructionScript`)