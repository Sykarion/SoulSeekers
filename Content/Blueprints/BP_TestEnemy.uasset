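; BP_TestEnemy is a test enemy Blueprint that links its floating health bar to itself.
; On BeginPlay it runs the parent logic, casts the HealthUI widget to WBP_FloatingHealthBar and sets itself as owner, printing an error if the cast fails.
; Overlap and Tick events are disabled stubs, and the construction script only calls the parent.
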(event `self.ReceiveBeginPlay`
  (`parent.ReceiveBeginPlay`)
  (bind _aswbp_floating_health_bar (cast `/Game/Blueprints/UI/WBP_FloatingHealthBar` (`WidgetComponent.GetWidget` (`self.Health_UI`)))
    (:`then`
      (`/Game/Blueprints/UI/WBP_FloatingHealthBar.SetOwner` _aswbp_floating_health_bar self))
    (:`CastFailed`
      (`KismetSystemLibrary.PrintString` "Can't find WBP_FloatingHealthBar"))))

(fn `UserConstructionScript`
  (`parent.UserConstructionScript`))