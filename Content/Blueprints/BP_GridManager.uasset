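; Grid manager actor that builds a tile grid and handles click-to-move for pawns on it.
; The construction script lays out static mesh placeholders as an editor preview, which BeginPlay destroys before GenerateGrid spawns tile actors into a coordinate-keyed map.
; HandleClick selects any clicked BPI_GridPawn, then sends it to a clicked BP_GridTile's coordinates and location through the interface and clears the selection.
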(event `self.ReceiveBeginPlay`
  (bind _editorgridtiles (`self.EditorGridTiles`))
  (for _array_element _editorgridtiles
    (`ActorComponent.K2_DestroyComponent` _array_element))
  (`KismetArrayLibrary.Array_Clear` _editorgridtiles)
  (`self.GenerateGrid`))

(event `HandleClick`
  (params (ClickedActor :type "Actor Object Reference"))
  (if (`KismetSystemLibrary.DoesImplementInterface` ClickedActor "/Game/Blueprints/Interfaces/BPI_GridPawn.BPI_GridPawn_C")
    (set `self.SelectedPawn` ClickedActor)
    (elif (`KismetSystemLibrary.IsValid` (`self.SelectedPawn`))
      (bind _asbp_grid_tile (cast `/Game/Blueprints/BP_GridTile` ClickedActor)
        (:`then`
          (message `/Game/Blueprints/Interfaces/BPI_GridPawn.MoveToGridCoords` (`self.SelectedPawn`) (`/Game/Blueprints/BP_GridTile.Position` _asbp_grid_tile) (`self.K2_GetActorLocation` _asbp_grid_tile))
          (set `self.SelectedPawn` null))
        (:`CastFailed`
          (set `self.SelectedPawn` null))))))

(fn `GenerateGrid`
  (bind _tilespacing (`self.TileSpacing`))
  (bind (_returnvalue_x _returnvalue_y) (break `IntPoint` (- (`self.GridSize`) (make `IntPoint` 1 1))))
  ;[1 1 1] x
  (for _index (range (+ _returnvalue_x 1))
    ;[1 1 1] y
    (for _index_2 (range (+ _returnvalue_y 1))
      (bind _intpoint (make `IntPoint` _index _index_2))
      (bind _returnvalue (`|SpawnActorFromClass` (`self.TileClass`) (`KismetMathLibrary.MakeTransform` (+ (`KismetMathLibrary.MakeVector` (* _index _tilespacing) (* _index_2 _tilespacing)) (`self.K2_GetActorLocation`))) "Undefined" "MultiplyWithRoot" null _intpoint null))
      (`BlueprintMapLibrary.Map_Add` (`self.GridTiles`) _intpoint _returnvalue))))

(fn `UserConstructionScript`
  (bind _tilespacing (`self.TileSpacing`))
  (bind (_returnvalue_x _returnvalue_y) (break `IntPoint` (- (`self.GridSize`) (make `IntPoint` 1 1))))
  (`KismetArrayLibrary.Array_Clear` (`self.EditorGridTiles`))
  ;[1 1 1] x
  (for _index (range (+ _returnvalue_x 1))
    ;[1 1 1] y
    (for _index_2 (range (+ _returnvalue_y 1))
      (bind _returnvalue (`AddComponent|NODE_AddStaticMeshComponent-1`))
      (`SceneComponent.K2_SetWorldTransform` _returnvalue (`KismetMathLibrary.MakeTransform` (+ (`KismetMathLibrary.MakeVector` (* _index _tilespacing) (* _index_2 _tilespacing)) (`self.K2_GetActorLocation`))) false false)
      (`KismetArrayLibrary.Array_Add` (`self.EditorGridTiles`) _returnvalue))))