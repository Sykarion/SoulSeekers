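; BP_RecoilObject is an actor whose static mesh plays a recoil punch with a highlight when R is pressed.
; BeginPlay enables input and caches the mesh's relative location as BaseLocation.
; The press normalizes BaseLocation minus the pawn's world location as the recoil direction, mixing relative and world space.
; The TL_RecoilPunch timeline offsets the mesh along that direction and drives the HighlightAmount material parameter.
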(event `self.ReceiveBeginPlay`
  (`self.EnableInput` (`GameplayStatics.GetPlayerController` 0))
  (bind _output_get (set `self.BaseLocation` (`SceneComponent.RelativeLocation` (`self.StaticMesh`)))))

(event `Key|R`
  (params (Key :type "Key Structure"))
  (:`Pressed`
    (bind _output_get (set `self.PawnLocation` (`self.K2_GetActorLocation` (`GameplayStatics.GetPlayerPawn` 0))))
    (bind _output_get_2 (set `self.Recoil Vector` (`KismetMathLibrary.Normal` (- (stale `self.ReceiveBeginPlay` _output_get) _output_get))))
    (bind (_direction _recoiloffset _highlightalpha) (`Timeline|TL_RecoilPunch` :!via `PlayFromStart`)
      (:`Update`
        (`MeshComponent.SetScalarParameterValueOnMaterials` (`self.StaticMesh`) "HighlightAmount" _highlightalpha)
        (`SceneComponent.K2_SetRelativeLocation` (`self.StaticMesh`) (+ (* (`KismetMathLibrary.Normal` _output_get_2) _recoiloffset) (`self.BaseLocation`)) false false)))))

(fn `UserConstructionScript`)