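; BP_FlipController is an actor meant to flip every actor tagged "Obstacles" around its own location when F is pressed.
; On BeginPlay it enables input, and each press stores the obstacles' start locations and targets rotated half a turn about the world Y axis.
; The FlipAnimation timeline loops over them on update, but the SetActorLocation lerp is disconnected, so nothing moves.
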(event `Key|F`
  (params (Key :type "Key Structure"))
  (bind _returnvalue (`self.K2_GetActorLocation`))
  (:`Pressed`
    (bind _outactors (`GameplayStatics.GetAllActorsWithTag` "Obstacles"))
    (set `self.ActorsToFlip` _outactors)
    (`KismetArrayLibrary.Array_Clear` (`self.StartLocation`))
    (`KismetArrayLibrary.Array_Clear` (`self.TargetLocation`))
    (for _array_element (`self.ActorsToFlip`)
      (`KismetArrayLibrary.Array_Add` (`self.StartLocation`) (`self.K2_GetActorLocation` _array_element))
      (`KismetArrayLibrary.Array_Add` (`self.TargetLocation`) (+ _returnvalue (`KismetMathLibrary.RotateAngleAxis` (- (`self.K2_GetActorLocation` _array_element) _returnvalue) 180.0 (0.0 1.0 0.0)))))
    (bind (_direction _alpha) (`Timeline|FlipAnimation` :!via `PlayFromStart`)
      (:`Update`
        (for (_array_element_2 _array_index) (`self.ActorsToFlip`)
          _)))))

(event `self.ReceiveBeginPlay`
  (`self.EnableInput` (`GameplayStatics.GetPlayerController` 0)))

(fn `UserConstructionScript`)