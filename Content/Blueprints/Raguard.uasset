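; Raguard is an actor Blueprint that turns in 90-degree yaw steps in response to player input.
; The Rotate Left action adds to a stored CurrentYaw and Rotate Right subtracts from it, truncating and wrapping the value with modulo 360.
; Each press snaps the actor to that yaw with zero pitch and roll, without interpolation, and prints a debug message.
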(event `InputAction|Rotate Left`
  (params (Key :type "Key Structure"))
  (:`Pressed`
    (bind _output_get (set `self.Current Yaw` (`KismetMathLibrary.Conv_IntToDouble` (mod (`KismetMathLibrary.FTrunc` (+ (`self.Current Yaw`) 90.0)) 360))))
    (`self.K2_SetActorRotation` (`KismetMathLibrary.MakeRotator` 0.0 0.0 _output_get))
    (`KismetSystemLibrary.PrintString` "pressed")))

(event `self.ReceiveTick`
  (params (DeltaSeconds :type "Float (single-precision)")))

(event `InputAction|Rotate Right`
  (params (Key :type "Key Structure"))
  (:`Pressed`
    (bind _output_get (set `self.Current Yaw` (`KismetMathLibrary.Conv_IntToDouble` (mod (`KismetMathLibrary.FTrunc` (- (`self.Current Yaw`) 90.0)) 360))))
    (`self.K2_SetActorRotation` (`KismetMathLibrary.MakeRotator` 0.0 0.0 _output_get))
    (`KismetSystemLibrary.PrintString` "pressed")))

(fn `UserConstructionScript`)